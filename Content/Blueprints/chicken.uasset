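; Player-controlled chicken pawn that moves in four directions and gets flattened when its mesh is overlapped.
; Direction actions rotate the actor and add movement input scaled by direction constants and MoveSpeed, which Tick applies as a swept local offset.
; A, D, Jump and touch set MoveSpeed, then stop it after a delay; releasing A or D stops it immediately.
; Impulse-based jump nodes are left unconnected.
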(event OnComponentBeginOverlap(StaticMesh)
  (params (OverlappedComponent :type Primitive%20Component%20Object%20Reference) (OtherActor :type Actor%20Object%20Reference) (OtherComp :type Primitive%20Component%20Object%20Reference) (OtherBodyIndex :type Integer) (bFromSweep :type Boolean) (SweepResult :type Hit%20Result%20Structure%20%28by%20ref%29))
  ;[1 1 1] kill chicken
  (Transformation|SetActorScale3D "0.250000,0.250000,0.100000"))

(event EventBeginPlay)

(event Collision|EventActorBeginOverlap
  (params (OtherActor :type Actor%20Object%20Reference)))

(event EventTick
  (params (DeltaSeconds :type Float%20%28single-precision%29))
  ;[1 1 1] Ticks
  (bind _returnvalue (Class|Pawn|ConsumeMovementInputVector))
  (Transformation|AddActorLocalOffset _returnvalue true false))

(event Input|ActionEvents|InputActionJump
  (params (Key :type Key%20Structure :default "None"))
  ;[1 1 1] coursework
  (:Pressed
    (Variables|Default|Setmove_speed (Variables|Default|Getbackwards))
    (Utilities|FlowControl|Delay 1.0)
    (Variables|Default|Setmove_speed (Variables|Default|Getstop))))

(event Input|ActionEvents|InputActionright
  (params (Key :type Key%20Structure :default "None"))
  ;[1 1 1] move right
  (:Pressed
    (Transformation|SetActorRotation "0,90.000000, 0")
    (Pawn|Input|AddMovementInput (Transformation|GetActorRightVector) (* (Variables|Default|Getbackwards) (Variables|Default|Getmove_speed)) false)))

(event Input|ActionEvents|InputActionforward
  (params (Key :type Key%20Structure :default "None"))
  ;[1 1 1] move forward
  (:Pressed
    (Transformation|SetActorRotation "0, 0, 0")
    (Pawn|Input|AddMovementInput (Transformation|GetActorForwardVector) (* (Variables|Default|Getforwards) (Variables|Default|Getmove_speed)) false)))

(event Input|ActionEvents|InputActionbackward
  (params (Key :type Key%20Structure :default "None"))
  ;[1 1 1] move backward
  (:Pressed
    (Transformation|SetActorRotation "0,180.000000, 0")
    (Pawn|Input|AddMovementInput (Transformation|GetActorForwardVector) (* (Variables|Default|Getbackwards) (Variables|Default|Getmove_speed)) false)))

(event Input|ActionEvents|InputActionleft
  (params (Key :type Key%20Structure :default "None"))
  ;[1 1 1] move left
  (:Pressed
    (Transformation|SetActorRotation "0,-90.000000, 0")
    (Pawn|Input|AddMovementInput (Transformation|GetActorRightVector) (* (Variables|Default|Getforwards) (Variables|Default|Getmove_speed)) false)))

(event Input|KeyboardEvents|A
  (params (Key :type Key%20Structure :default "None"))
  ;[1 1 1] coursework
  (:Pressed
    (Variables|Default|Setmove_speed (Variables|Default|Getbackwards))
    (Utilities|FlowControl|Delay 1.0)
    (Variables|Default|Setmove_speed (Variables|Default|Getstop) :!label _label))
  (:Released
    (Input|EnableInput 0)
    (goto _label)))

(event Input|KeyboardEvents|D
  (params (Key :type Key%20Structure :default "None"))
  ;[1 1 1] coursework
  (:Pressed
    (Variables|Default|Setmove_speed (Variables|Default|Getforwards))
    (Utilities|FlowControl|Delay 1.0)
    (Variables|Default|Setmove_speed (Variables|Default|Getstop) :!label _label))
  (:Released
    (Input|EnableInput 0)
    (goto _label)))

(event Input|TouchEvents|InputTouch
  (params (Location :type Vector) (FingerIndex :type ETouchIndex%20Enum))
  ;[1 1 1] coursework
  (:Pressed
    (Variables|Default|Setmove_speed (Variables|Default|Getbackwards))
    (Utilities|FlowControl|Delay 1.0)
    (Variables|Default|Setmove_speed (Variables|Default|Getstop))))

(fn ConstructionScript)